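; Two-floor cabin that serves as a streamed-level transition, with scripted doors, fixed interior cameras and Wwise footstep switching.
; BeginPlay picks door trigger boxes and starting camera from spawn/entry flags; Tick polls box overlaps to drive everything.
; Door timelines chain so one opening closes the other and swaps streamed levels, depending on entry flags.
; View-target blends switch between player and cabin cameras, pausing mouse input, while paired stair triggers toggle upper and lower views.
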(event EventBeginPlay
  ;[1 1 1] Begin
  (Variables|Default|SetPlayer (Game|GetPlayerCharacter 0))
  (Variables|Default|SetRotDoor1 (Transformation|GetWorldRotation (Variables|Default|GetDoor1)))
  (Variables|Default|SetRotDoor2 (Transformation|GetWorldRotation (Variables|Default|GetDoor2)))
  (if (Variables|Default|GetLS_SpawnedFromTop)
    (Variables|Default|SetDoor2%20Opened true)
    (Variables|Default|SetBoxColisionDoor1 (Variables|Default|GetBox2-2))
    (Variables|Default|SetBoxColisionDoor2 (Variables|Default|GetBox1-2))
    (Game|Player|SetViewTargetwithBlend (Game|GetPlayerController 0) (Components|GetOwner (Variables|Default|GetCameraUp)) 0.0 "VTBlend_Linear" 0.0 false)
    (Variables|Default|SetUpperCamera true)
    (Components|Activation|Activate (Variables|Default|GetCameraUp) false)
    (Components|Activation|Deactivate (Variables|Default|GetCameraDown))
    (elif (Variables|Default|GetLS_SpawnedFromBot)
      (Variables|Default|SetBoxColisionDoor1 (Variables|Default|GetBox2-1))
      (Variables|Default|SetBoxColisionDoor2 (Variables|Default|GetBox1-1))
      (Game|Player|SetViewTargetwithBlend (Game|GetPlayerController 0) (Components|GetOwner (Variables|Default|GetCameraDown)) 0.0 "VTBlend_Linear" 0.0 false)
      (Variables|Default|SetUpperCamera false)
      (Components|Activation|Activate (Variables|Default|GetCameraDown) false)
      (Components|Activation|Deactivate (Variables|Default|GetCameraUp))
      (else
        (if (Variables|Default|GetnoLS_EnterFromBot)
          (Variables|Default|SetBoxColisionDoor1 (Variables|Default|GetBox1-1))
          (Variables|Default|SetBoxColisionDoor2 (Variables|Default|GetBox2-1))
          (else
            (Variables|Default|SetBoxColisionDoor1 (Variables|Default|GetBox1-2))
            (Variables|Default|SetBoxColisionDoor2 (Variables|Default|GetBox2-2))))
        (Components|Activation|Activate (Variables|Default|GetCameraDown) false)
        (Components|Activation|Deactivate (Variables|Default|GetCameraUp))
        (Variables|Default|SetExit true)))))

(event EventTick
  (params (DeltaSeconds :type Float%20%28single-precision%29))
  (bind _rotdoor2 (Variables|Default|GetRotDoor2))
  (bind _cabin (Variables|Default|GetCabin))
  (bind _rotdoor1 (Variables|Default|GetRotDoor1))
  (bind (_roll _pitch _yaw) (Math|Rotator|BreakRotator _rotdoor1))
  (bind (_roll_2 _pitch_2 _yaw_2) (Math|Rotator|BreakRotator _rotdoor2))
  (bind _returnvalue (Transformation|GetWorldRotation _cabin))
  (bind (_roll_3 _pitch_3 _yaw_3) (Math|Rotator|BreakRotator _returnvalue))
  ;[1 1 1] FootStepManager
  (if (Collision|IsOverlappingActor (Variables|Default|GetFootStepTrigger) (Variables|Default|GetPlayer) :!class /Script/Engine.PrimitiveComponent)
    (if (Variables|Default|GetisFoostepWood)
      _
      (else
        (bind _asthird_person_character (Utilities|Casting|CastToThirdPersonCharacter (Variables|Default|GetPlayer)))
        (bind _returnvalue_2 (Class|AkGameplayStatics|GetAkComponent (Variables|/Script/Engine.Character|GetMesh _asthird_person_character) "None" "0, 0, 0" "KeepRelativeOffset"))
        (Class|AkComponent|SetSwitch _returnvalue_2 "Footsteps" "Wood")
        (Variables|Default|SetisFoostepWood true)))
    (elif (Variables|Default|GetisFoostepWood)
      (bind _asthird_person_character_2 (Utilities|Casting|CastToThirdPersonCharacter (Variables|Default|GetPlayer)))
      (bind _returnvalue_3 (Class|AkGameplayStatics|GetAkComponent (Variables|/Script/Engine.Character|GetMesh _asthird_person_character_2) "None" "0, 0, 0" "KeepRelativeOffset"))
      (Class|AkComponent|SetSwitch _returnvalue_3 "Footsteps" "Dirt")
      (Variables|Default|SetisFoostepWood false)))
  (if (Variables|Default|GetExit)
    ;[1 1 1] Enter from the bot after an Exit
    (if (Collision|IsOverlappingActor (Variables|Default|GetBox1-3) (Variables|Default|GetPlayer) :!class /Script/Engine.PrimitiveComponent)
      (Game|Player|SetViewTargetwithBlend (Game|GetPlayerController 0) (Components|GetOwner (Variables|Default|GetCameraDown)) 1.0 "VTBlend_EaseInOut" 1.0 false)
      (Components|Activation|Activate (Variables|Default|GetCameraDown) false)
      (Components|Activation|Deactivate (Variables|Default|GetCameraUp))
      (Variables|Default|SetUpperCamera false)
      (Variables|Default|SetCamDoor1Passed false :!label _label)
      (Variables|Default|SetCamDoor2Passed false)
      (Variables|Default|SetExit false)
      (Variables|Default|SetEnter true)
      (Timeline|Timeline_0 PlayFromStart
        (:Update
          (bind _asthird_person_character_3 (Utilities|Casting|CastToThirdPersonCharacter (Variables|Default|GetPlayer)))
          (Variables|/Game/MainCharacter/Blueprints/ThirdPersonCharacter.ThirdPersonCharacter_C|Setmouse _asthird_person_character_3 false))
        (:Finished
          (bind _asthird_person_character_4 (Utilities|Casting|CastToThirdPersonCharacter (Variables|Default|GetPlayer)))
          (Variables|/Game/MainCharacter/Blueprints/ThirdPersonCharacter.ThirdPersonCharacter_C|Setmouse _asthird_person_character_4 true)
          (Variables|Default|SetEnter false)))
      (else
        ;[1 1 1] Enter from the Top after an Exit
        (if (Collision|IsOverlappingActor (Variables|Default|GetBox2-1) (Variables|Default|GetPlayer) :!class /Script/Engine.PrimitiveComponent)
          (Game|Player|SetViewTargetwithBlend (Game|GetPlayerController 0) (Components|GetOwner (Variables|Default|GetCameraUp)) 1.0 "VTBlend_EaseInOut" 1.0 false)
          (Components|Activation|Activate (Variables|Default|GetCameraUp) false)
          (Components|Activation|Deactivate (Variables|Default|GetCameraDown))
          (Variables|Default|SetUpperCamera true)
          (goto _label)
          (else
            (if (or (Variables|Default|GetLS_SpawnedFromTop) (Variables|Default|GetLS_SpawnedFromBot)) :!label _label_2
              ;[1 1 1] Scripted Doors After Loading Scene
              (if (Variables|Default|GetLS_SpawnedFromTop)
                (Variables|Default|SetDoor1%20Opened true)
                ;[1 1 1] Open Door 2
                (bind _newtrack_0 (Timeline|OpenDoor2 Play)
                  (:Update
                    (Transformation|SetWorldRotation (Variables|Default|GetDoor2) (Math|Rotator|MakeRotator _roll_2 _pitch_2 (+ _yaw_2 _newtrack_0)) false false)
                    (if (not (Variables|Default|GetDoor2%20Opened))
                      (Variables|Default|SetDoor2%20Opened true)
                      (if (not (Class|TimelineComponent|IsReversing (Variables|Default|GetOpenDoor1)))
                        ;;[1 1 1] Close the other Door
                        (if (Variables|Default|GetnoLS_EnterFromBot)
                          (Game|LoadStreamLevel(byName) (Variables|Default|GetLoad%20Level) true)
                          (Game|UnloadStreamLevel(byName) (Variables|Default|GetUnload%20Level))
                          (Game|LoadStreamLevel(byName) (Variables|Default|GetCabinLoad) true)
                          (if (Variables|Default|GetisFoostepWood)
                            ;;[1 1 1] make sure wood noise are enabled
                            (bind _asthird_person_character_5 (Utilities|Casting|CastToThirdPersonCharacter (Variables|Default|GetPlayer)))
                            (bind _returnvalue_4 (Class|AkGameplayStatics|GetAkComponent (Variables|/Script/Engine.Character|GetMesh _asthird_person_character_5) "None" "0, 0, 0" "KeepRelativeOffset"))
                            (Class|AkComponent|SetSwitch _returnvalue_4 "Footsteps" "Wood"))
                          (Class|AkGameplayStatics|PostEventatLocation 0 (Transformation|GetWorldLocation (Variables|Default|GetDoor1)) "0, 0, 0")
                          ;[1 1 1] Open Door 1
                          (bind _newtrack_0_2 (Timeline|OpenDoor1 Reverse)
                            (:Update
                              (Transformation|SetWorldRotation (Variables|Default|GetDoor1) (Math|Rotator|MakeRotator _roll _pitch (+ _yaw _newtrack_0_2)) false false)
                              (if (not (Variables|Default|GetDoor1%20Opened))
                                (Variables|Default|SetDoor1%20Opened true)
                                (if (not (Class|TimelineComponent|IsReversing (Variables|Default|GetOpenDoor2)))
                                  ;;[1 1 1] Close the other Door
                                  (if (Variables|Default|GetnoLS_EnterFromTop)
                                    (Game|LoadStreamLevel(byName) (Variables|Default|GetLoad%20Level) true)
                                    (Game|UnloadStreamLevel(byName) (Variables|Default|GetUnload%20Level))
                                    (Game|UnloadStreamLevel(byName) (Variables|Default|GetCabinLoad))
                                    (if (Variables|Default|GetisFoostepWood)
                                      ;;[1 1 1] make sure wood noise are enabled
                                      (bind _asthird_person_character_6 (Utilities|Casting|CastToThirdPersonCharacter (Variables|Default|GetPlayer)))
                                      (bind _returnvalue_5 (Class|AkGameplayStatics|GetAkComponent (Variables|/Script/Engine.Character|GetMesh _asthird_person_character_6) "None" "0, 0, 0" "KeepRelativeOffset"))
                                      (Class|AkComponent|SetSwitch _returnvalue_5 "Footsteps" "Wood"))
                                    (Class|AkGameplayStatics|PostEventatLocation 0 (Transformation|GetWorldLocation (Variables|Default|GetDoor2)) "0, 0, 0")
                                    (Timeline|OpenDoor2 Reverse)))))))))))
                (else
                  (Variables|Default|SetDoor2%20Opened true)
                  (Timeline|OpenDoor1 Play)))
              (elif (Variables|Default|GetDoor1%20Opened)
                (if (not (Variables|Default|GetDoor2%20Opened))
                  ;;[1 1 1] Enter From Top
                  (if (Collision|IsOverlappingActor (Variables|Default|GetBoxColisionDoor2) (Variables|Default|GetPlayer) :!class /Script/Engine.PrimitiveComponent) :!label _label_3
                    (if (not (Variables|Default|GetDoor2%20Opened))
                      (Class|AkGameplayStatics|PostEventatLocation "/Game/Wwise/Play_Door_open.Play_Door_open" (Transformation|GetWorldLocation (Variables|Default|GetDoor2)) "0, 0, 0")
                      (Timeline|OpenDoor2 Play))))
                (elif (Collision|IsOverlappingActor (Variables|Default|GetBoxColisionDoor1) (Variables|Default|GetPlayer) :!class /Script/Engine.PrimitiveComponent)
                  (if (not (Variables|Default|GetDoor1%20Opened))
                    (Class|AkGameplayStatics|PostEventatLocation "/Game/Wwise/Play_Door_open.Play_Door_open" (Transformation|GetWorldLocation (Variables|Default|GetDoor1)) "0, 0, 0")
                    (Timeline|OpenDoor1 Play))
                  (else
                    (goto _label_3)))))))))
    (elif (not (Variables|Default|GetEnter))
      (if (or (Variables|Default|GetLS_SpawnedFromBot) (Variables|Default|GetnoLS_EnterFromTop))
        (if (Collision|IsOverlappingActor (Variables|Default|GetBox1-1) (Variables|Default|GetPlayer) :!class /Script/Engine.PrimitiveComponent) :!label _label_4
          ;[1 1 1] Exit Camera Rotation From 1st Floor
          (Pawn|SetControlRotation (Game|GetPlayerController 0) (Math|Rotator|MakeRotator 0.0 (- _pitch_3 5.0) (+ _yaw_3 9e+01)))
          ;[1 1 1] Exit/Enter
          (Game|Player|SetViewTargetwithBlend (Game|GetPlayerController 0) (Pawn|GetControlledPawn (Game|GetPlayerController 0)) 1.0 "VTBlend_EaseInOut" 1.0 false :!label _label_5)
          (Variables|Default|SetExit true)
          (Timeline|WaitingForBlend PlayFromStart
            (:Update
              (bind _asthird_person_character_7 (Utilities|Casting|CastToThirdPersonCharacter (Variables|Default|GetPlayer)))
              (Variables|/Game/MainCharacter/Blueprints/ThirdPersonCharacter.ThirdPersonCharacter_C|Setmouse _asthird_person_character_7 false))
            (:Finished
              (bind _asthird_person_character_8 (Utilities|Casting|CastToThirdPersonCharacter (Variables|Default|GetPlayer)))
              (Variables|/Game/MainCharacter/Blueprints/ThirdPersonCharacter.ThirdPersonCharacter_C|Setmouse _asthird_person_character_8 true)
              (Variables|Default|SetPlayer (Game|GetPlayerCharacter 0))))
          (else
            (if (and (Variables|Default|GetDoor2%20Opened) (not (Variables|Default|GetDoor1%20Opened)))
              (if (Collision|IsOverlappingActor (Variables|Default|GetBox2-2) (Variables|Default|GetPlayer) :!class /Script/Engine.PrimitiveComponent) :!label _label_6
                ;[1 1 1] Exit Camera Rotation From 2nd Floor
                (Pawn|SetControlRotation (Game|GetPlayerController 0) (Math|Rotator|MakeRotator 0.0 0.0 (+ (.Yaw (Math|Rotator|BreakRotator (Transformation|GetWorldRotation (Variables|Default|GetCabin)))) -9e+01)))
                (goto _label_5)
                (elif (and (Variables|Default|GetDoor1%20Opened) (not (Variables|Default|GetDoor2%20Opened)))
                  (goto _label_4)
                  (else
                    _))))
            ;[1 1 1] Camera Trigger Up and Down
            (if (and (Collision|IsOverlappingActor (Variables|Default|GetStairsCameraTrigger1) (Variables|Default|GetPlayer) :!class /Script/Engine.PrimitiveComponent) (not (Variables|Default|GetCamDoor2Passed)))
              (Variables|Default|SetCamDoor1Passed true))
            (if (Variables|Default|GetCamDoor1Passed)
              (if (Collision|IsOverlappingActor (Variables|Default|GetStairsCameraTrigger2) (Variables|Default|GetPlayer) :!class /Script/Engine.PrimitiveComponent)
                _
                (else
                  (goto _label_2)))
              (else
                (if (and (Collision|IsOverlappingActor (Variables|Default|GetStairsCameraTrigger2) (Variables|Default|GetPlayer) :!class /Script/Engine.PrimitiveComponent) (not (Variables|Default|GetCamDoor1Passed)))
                  (Variables|Default|SetCamDoor2Passed true))
                (if (Variables|Default|GetCamDoor2Passed)
                  (if (Collision|IsOverlappingActor (Variables|Default|GetStairsCameraTrigger1) (Variables|Default|GetPlayer) :!class /Script/Engine.PrimitiveComponent)
                    _
                    (else
                      (goto _label_2)))
                  (else
                    (goto _label_2)))))
            (if (Variables|Default|GetUpperCamera)
              ;[1 1 1] Camera Switch
              (Game|Player|SetViewTargetwithBlend (Game|GetPlayerController 0) (Components|GetOwner (Variables|Default|GetCameraDown)) 0.0 "VTBlend_Linear" 0.0 false)
              (Variables|Default|SetUpperCamera false)
              (Components|Activation|Activate (Variables|Default|GetCameraDown) false)
              (Components|Activation|Deactivate (Variables|Default|GetCameraUp))
              (else
                (Game|Player|SetViewTargetwithBlend (Game|GetPlayerController 0) (Components|GetOwner (Variables|Default|GetCameraUp)) 0.0 "VTBlend_Linear" 0.0 false)
                (Variables|Default|SetUpperCamera true)
                (Components|Activation|Deactivate (Variables|Default|GetCameraDown))
                (Components|Activation|Activate (Variables|Default|GetCameraUp) false)))
            (Variables|Default|SetCamDoor1Passed false)
            (Variables|Default|SetCamDoor2Passed false)))
        (else
          (goto _label_6))))))

(fn ConstructionScript)