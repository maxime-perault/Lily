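; BP_DoorBF is a boss fight door that shuts once when the player character enters its trigger.
; Construction disables the closed-door collision, leaving the passage open until triggered.
; The overlap disables the trigger, posts the Wwise event BlackDoor_Open at the door, then calls Close.
; Close enables the blocking collision and plays the door animation once, with no logic to reopen it.
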(event OnComponentBeginOverlap(Trigger)
  (params (OverlappedComponent :type Primitive%20Component%20Object%20Reference) (OtherActor :type Actor%20Object%20Reference) (OtherComp :type Primitive%20Component%20Object%20Reference) (OtherBodyIndex :type Integer) (bFromSweep :type Boolean) (SweepResult :type Hit%20Result%20Structure%20%28by%20ref%29))
  (if (== (Game|GetPlayerCharacter 0) OtherActor)
    (Collision|SetCollisionEnabled (Variables|Default|GetTrigger) "NoCollision")
    (Class|AkGameplayStatics|PostEventatLocation "/Game/Wwise/BlackDoor_Open.BlackDoor_Open" (Transformation|GetWorldLocation (Variables|Default|GetDoorClosedCollision)) "0, 0, 0")
    (CallFunction|Close)))

(fn ConstructionScript
  (Collision|SetCollisionEnabled (Variables|Default|GetDoorClosedCollision) "NoCollision"))

(fn Close
  (Collision|SetCollisionEnabled (Variables|Default|GetDoorClosedCollision) "QueryAndPhysics")
  (Components|Animation|PlayAnimation (Variables|Default|GetEnv_BossDoor) "/Game/Environment/DoorBF/Env_BossDoor_Anim.Env_BossDoor_Anim" false))