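; Boss-fight trigger that sends Psychosis dashing through a chain of target positions when the player enters, then disables its collision.
; The construction script grabs the first BP_Psychosis; the overlap event loops through NextPosArray, pausing briefly before later hops.
; Each hop hides the boss via the Mpc_dash parameter collection, plays sound, spawns a ghost and particles, and lerps location on a timeline.
; On arrival it matches rotation, reappears, and a second timeline gates the next hop.
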(event OnComponentBeginOverlap(Trigger)
  (params (OverlappedComponent :type Primitive%20Component%20Object%20Reference) (OtherActor :type Actor%20Object%20Reference) (OtherComp :type Primitive%20Component%20Object%20Reference) (OtherBodyIndex :type Integer) (bFromSweep :type Boolean) (SweepResult :type Hit%20Result%20Structure%20%28by%20ref%29))
  (bind _psychosis (Variables|Default|GetPsychosis))
  (if (== (Game|GetPlayerCharacter 0) OtherActor)
    (Collision|SetCollisionEnabled (Variables|Default|GetTrigger) "NoCollision")
    (if (< (Variables|Default|Getindex) (Utilities|Array|Length (Variables|Default|GetNextPosArray))) :!label _label
      (if (> (Variables|Default|Getindex) 1)
        (Utilities|FlowControl|Delay 0.3))
      (Variables|Default|SetNextPos (Utilities|Array|Get(acopy) (Variables|Default|GetNextPosArray) (Variables|Default|Getindex)))
      (Math|Integer|IncrementInt (Variables|Default|Getindex)
        (:%20%20
          (Variables|Default|SetCurrentLocation (Transformation|GetWorldLocation (Variables|/Game/DarkPhase/Psychosis/BP_Psychosis.BP_Psychosis_C|GetSkeletalMesh (Variables|Default|GetPsychosis))))
          (Rendering|Material|SetScalarParameterValue "/Game/Effects/DashingEffect/mpc_dash.mpc_dash" "PsychosisVisible" 0.0 :!class /Script/Engine.KismetMaterialLibrary)
          (Class|AkGameplayStatics|PostEvent "/Game/Wwise/Boss_Dash.Boss_Dash" _psychosis false)
          (Game|SpawnActorfromClass "/Game/Effects/DashingEffect/BP_Ghost_Psycho.BP_Ghost_Psycho_C" (Transformation|GetActorTransform _psychosis) "Undefined" 0 0)
          (bind _returnvalue (AddComponent|AddParticleSystemComponent _psychosis false))
          (Effects|Components|ParticleSystem|SetActorParameter _returnvalue "VertSurfaceActor" _psychosis)
          (bind _newtrack_0 (Timeline|WaitVisible PlayFromStart)
            (:Update
              (Transformation|SetActorLocation (Variables|Default|GetPsychosis) (Math|Vector|Lerp(Vector) (Variables|Default|GetCurrentLocation) (Transformation|GetWorldLocation (Variables|/Script/Engine.Actor|GetRootComponent (Variables|Default|GetNextPos))) _newtrack_0) false true))
            (:Finished
              (Transformation|SetActorRotation (Variables|Default|GetPsychosis) (Transformation|GetWorldRotation (Variables|/Script/Engine.Actor|GetRootComponent (Variables|Default|GetNextPos))) true)
              (Rendering|Material|SetScalarParameterValue "/Game/Effects/DashingEffect/mpc_dash.mpc_dash" "PsychosisVisible" 1.0 :!class /Script/Engine.KismetMaterialLibrary)
              (Timeline|WaitParticle PlayFromStart
                (:Finished
                  (goto _label))))))))))

(fn ConstructionScript
  (bind _outactors (Actor|GetAllActorsOfClass "/Game/DarkPhase/Psychosis/BP_Psychosis.BP_Psychosis_C"))
  (Variables|Default|SetPsychosis (Utilities|Array|Get(acopy) _outactors)))