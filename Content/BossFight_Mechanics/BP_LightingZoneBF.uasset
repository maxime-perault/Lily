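; BP_LightingZoneBF is a boss-fight lighting zone pairing a spotlight with a sphere collision that shrink and grow together.
; Construction caches the sphere radius, cone angles and intensity as baselines.
; Decrease and Increase set flags that Tick consumes to play one timeline forward or in reverse.
; The timeline scales radius and cones by one curve and intensity by another; the sphere's begin-overlap event is empty.
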(event OnComponentBeginOverlap(Sphere)
  (params (OverlappedComponent :type Primitive%20Component%20Object%20Reference) (OtherActor :type Actor%20Object%20Reference) (OtherComp :type Primitive%20Component%20Object%20Reference) (OtherBodyIndex :type Integer) (bFromSweep :type Boolean) (SweepResult :type Hit%20Result%20Structure%20%28by%20ref%29)))

(event EventTick
  (params (DeltaSeconds :type Float%20%28single-precision%29))
  (bind _spotlight (Variables|Default|GetSpotLight))
  (if (Variables|Default|Getdown)
    (Variables|Default|Setdown false)
    (bind (_direction _scale _itensity_scale) (Timeline|DecreaseLightingZone PlayFromStart)
      (:Update
        (Components|Sphere|SetSphereRadius (Variables|Default|GetSphere) (* (Variables|Default|Getsphere_radius) _scale) true)
        (Rendering|Lighting|SetOuterConeAngle _spotlight (* (Variables|Default|Getouter_cone) _scale))
        (Rendering|Lighting|SetInnerConeAngle _spotlight (* (Variables|Default|Getinner_cone) _scale))
        (Rendering|Components|Light|SetIntensity _spotlight (* (Variables|Default|Getintensity) _itensity_scale))))
    (elif (Variables|Default|Getup)
      (Variables|Default|Setup false)
      (Timeline|DecreaseLightingZone ReverseFromEnd))))

(fn ConstructionScript
  (bind _spotlight (Variables|Default|GetSpotLight))
  (Variables|Default|Setouter_cone (Variables|/Script/Engine.SpotLightComponent|GetOuterConeAngle _spotlight))
  (Variables|Default|Setintensity (Variables|/Script/Engine.LightComponentBase|GetIntensity _spotlight))
  (Variables|Default|Setinner_cone (Variables|/Script/Engine.SpotLightComponent|GetInnerConeAngle _spotlight))
  (Variables|Default|Setsphere_radius (Variables|/Script/Engine.SphereComponent|GetSphereRadius (Variables|Default|GetSphere))))

(fn Decrease
  (Variables|Default|Setdown true))

(fn Increase
  (Variables|Default|Setup true))