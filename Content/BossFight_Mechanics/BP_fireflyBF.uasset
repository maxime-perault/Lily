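; Boss fight firefly pickup that the player triggers by overlap to call Decrease on its assigned lighting zones.
; The construction script caches the light intensity and spawns orbiting fireflies, using the green particle template when IsPermanent is set.
; On player overlap it disables the trigger, hides the particles, zeroes the light and loops through ArrayLightingZone, with an optional Delay before each zone after the first.
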(event OnComponentBeginOverlap(Trigger)
  (params (OverlappedComponent :type Primitive%20Component%20Object%20Reference) (OtherActor :type Actor%20Object%20Reference) (OtherComp :type Primitive%20Component%20Object%20Reference) (OtherBodyIndex :type Integer) (bFromSweep :type Boolean) (SweepResult :type Hit%20Result%20Structure%20%28by%20ref%29))
  (if (== (Game|GetPlayerCharacter 0) OtherActor)
    (Collision|SetCollisionEnabled (Variables|Default|GetTrigger) "NoCollision")
    (Rendering|SetVisibility (Variables|Default|GetFirefly) false false)
    (Rendering|Components|Light|SetIntensity (Variables|Default|GetPointLight) 0.0)
    (for (_array_element _array_index) (Variables|Default|GetArray_LightingZone)
      (if (and (Variables|Default|GetisTimerBetweenZones) (!= _array_index 0))
        (Utilities|FlowControl|Delay (Variables|Default|GetTimerBetweenZones)))
      (Default|Decrease _array_element))))

(fn ConstructionScript
  (Variables|Default|SetLight%20Intensity (Variables|/Script/Engine.LightComponentBase|GetIntensity (Variables|Default|GetPointLight)))
  (if (Variables|Default|GetisPermanent)
    (bind _returnvalue (AddComponent|AddParticleSystemComponent false))
    (Effects|Components|ParticleSystem|SetTemplate _returnvalue "/Game/DarkPhase/Fireflies/P_orbitFireflies_Green.P_orbitFireflies_Green")
    (Variables|Default|SetFirefly _returnvalue)
    (else
      (bind _returnvalue_2 (AddComponent|AddParticleSystemComponent false))
      (Effects|Components|ParticleSystem|SetTemplate _returnvalue_2 "/Game/DarkPhase/Fireflies/P_orbitFireflies.P_orbitFireflies")
      (Variables|Default|SetFirefly _returnvalue_2))))