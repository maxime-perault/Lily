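; Boss fight trigger actor that advances the music state as the player reaches each of four switch volumes.
; Each switch reacts only to the player character's overlap and sets the MUSIC_State group to its own phase, from P2 through P5.
; A triggered switch turns off its own collision so it fires once, and nothing in the graph enforces the order.
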(event OnComponentBeginOverlap(switch1)
  (params (OverlappedComponent :type Primitive%20Component%20Object%20Reference) (OtherActor :type Actor%20Object%20Reference) (OtherComp :type Primitive%20Component%20Object%20Reference) (OtherBodyIndex :type Integer) (bFromSweep :type Boolean) (SweepResult :type Hit%20Result%20Structure%20%28by%20ref%29))
  (if (== OtherActor (Game|GetPlayerCharacter 0))
    (Collision|SetCollisionEnabled (Variables|Default|Getswitch1) "NoCollision")
    (Class|AkGameplayStatics|SetState "MUSIC_State" "P2")))

(event OnComponentBeginOverlap(switch2)
  (params (OverlappedComponent :type Primitive%20Component%20Object%20Reference) (OtherActor :type Actor%20Object%20Reference) (OtherComp :type Primitive%20Component%20Object%20Reference) (OtherBodyIndex :type Integer) (bFromSweep :type Boolean) (SweepResult :type Hit%20Result%20Structure%20%28by%20ref%29))
  (if (== OtherActor (Game|GetPlayerCharacter 0))
    (Collision|SetCollisionEnabled (Variables|Default|Getswitch2) "NoCollision")
    (Class|AkGameplayStatics|SetState "MUSIC_State" "P3")))

(event OnComponentBeginOverlap(switch3)
  (params (OverlappedComponent :type Primitive%20Component%20Object%20Reference) (OtherActor :type Actor%20Object%20Reference) (OtherComp :type Primitive%20Component%20Object%20Reference) (OtherBodyIndex :type Integer) (bFromSweep :type Boolean) (SweepResult :type Hit%20Result%20Structure%20%28by%20ref%29))
  (if (== OtherActor (Game|GetPlayerCharacter 0))
    (Collision|SetCollisionEnabled (Variables|Default|Getswitch3) "NoCollision")
    (Class|AkGameplayStatics|SetState "MUSIC_State" "P4")))

(event OnComponentBeginOverlap(switch4)
  (params (OverlappedComponent :type Primitive%20Component%20Object%20Reference) (OtherActor :type Actor%20Object%20Reference) (OtherComp :type Primitive%20Component%20Object%20Reference) (OtherBodyIndex :type Integer) (bFromSweep :type Boolean) (SweepResult :type Hit%20Result%20Structure%20%28by%20ref%29))
  (if (== OtherActor (Game|GetPlayerCharacter 0))
    (Collision|SetCollisionEnabled (Variables|Default|Getswitch4) "NoCollision")
    (Class|AkGameplayStatics|SetState "MUSIC_State" "P5")))

(fn ConstructionScript)