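; One-shot trigger actor that switches the level's mood to a cool, foggy, dimly lit look with its own soundscape.
; The first overlap by any actor sets a Triggered flag and calls PlaySoundscapeS1 on the player's ThirdPersonCharacter.
; It then instantly overwrites settings on referenced post-process volume, height fog, directional light and skylight actors with hardcoded values, without blending.
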(event Collision|EventActorBeginOverlap
  (params (OtherActor :type Actor%20Object%20Reference))
  (if (not (Variables|Default|Gettriggered))
    (Variables|Default|Settriggered true)
    (bind _asthird_person_character (Utilities|Casting|CastToThirdPersonCharacter (Game|Player|GetPlayerPawn 0)))
    (Default|PlaySoundscapeS1 _asthird_person_character)
    ;[1 1 1] Post Process Volume
    (bind _aspost_process_volume (Utilities|Casting|CastToPostProcessVolume (Variables|Default|GetPostProcessVolume)))
    (Utilities|Struct|SetmembersinPostProcessSettings (Variables|/Script/Engine.PostProcessVolume|GetSettings _aspost_process_volume) 2.7e+03 -0.7 (Math|Vector4|MakeVector4 0.0 0.11 0.24 1.15) (Math|Vector4|MakeVector4 1.0 1.0 1.0 1.0) (Math|Vector4|MakeVector4 1.1 1.2 1.2 0.5) 2.5 0.0 0.0 0.7 0.0 0.05)
    ;[1 1 1] HeightFog
    (bind _asexponential_height_fog (Utilities|Casting|CastToExponentialHeightFog (Variables|Default|GetHeightFog)))
    (Class|ExponentialHeightFogComponent|SetFogInscatteringColor (Variables|/Script/Engine.ExponentialHeightFog|GetComponent _asexponential_height_fog) (Utilities|Struct|MakeLinearColor 0.76 1.0 0.94 1.0))
    (Class|ExponentialHeightFogComponent|SetFogDensity (Variables|/Script/Engine.ExponentialHeightFog|GetComponent _asexponential_height_fog) 0.9)
    (Class|ExponentialHeightFogComponent|SetFogHeightFalloff (Variables|/Script/Engine.ExponentialHeightFog|GetComponent _asexponential_height_fog) 0.2)
    (Class|ExponentialHeightFogComponent|SetStartDistance (Variables|/Script/Engine.ExponentialHeightFog|GetComponent _asexponential_height_fog) 0.0)
    (Class|ExponentialHeightFogComponent|SetDirectionalInscatteringStartDistance (Variables|/Script/Engine.ExponentialHeightFog|GetComponent _asexponential_height_fog) 1e+02)
    (Class|ExponentialHeightFogComponent|SetDirectionalInscatteringColor (Variables|/Script/Engine.ExponentialHeightFog|GetComponent _asexponential_height_fog) (Utilities|Struct|MakeLinearColor 0.02 0.06 0.25 1.0))
    (Class|ExponentialHeightFogComponent|SetVolumetricFogScatteringDistribution (Variables|/Script/Engine.ExponentialHeightFog|GetComponent _asexponential_height_fog) 0.11)
    (Class|ExponentialHeightFogComponent|SetVolumetricFogEmissive (Variables|/Script/Engine.ExponentialHeightFog|GetComponent _asexponential_height_fog) (Math|Conversions|ToLinearColor(Color) (Math|Color|MakeColor 0 0 0 1)))
    (Class|ExponentialHeightFogComponent|SetVolumetricFogExtinctionScale (Variables|/Script/Engine.ExponentialHeightFog|GetComponent _asexponential_height_fog) 1.2)
    (Class|ExponentialHeightFogComponent|SetVolumetricFogDistance (Variables|/Script/Engine.ExponentialHeightFog|GetComponent _asexponential_height_fog) 1.2e+03)
    (Class|ExponentialHeightFogComponent|SetVolumetricFog (Variables|/Script/Engine.ExponentialHeightFog|GetComponent _asexponential_height_fog) false)
    ;[1 1 1] Directional Light
    (bind _asdirectional_light (Utilities|Casting|CastToDirectionalLight (Variables|Default|GetLightSource)))
    (Rendering|Components|Light|SetIntensity (Variables|/Script/Engine.Light|GetLightComponent _asdirectional_light) 2.6)
    (Rendering|Components|Light|SetLightColor (Variables|/Script/Engine.Light|GetLightComponent _asdirectional_light) (Utilities|Struct|MakeLinearColor 0.527115 0.806952 1.0 1.0) true)
    ;[1 1 1] SkyLight
    (bind _assky_light (Utilities|Casting|CastToSkyLight (Variables|Default|GetSkyLight)))
    (Rendering|Components|Light|SetIntensity (Variables|/Script/Engine.SkyLight|GetLightComponent _assky_light) 0.19)
    (Rendering|Components|Light|SetLightColor (Variables|/Script/Engine.SkyLight|GetLightComponent _assky_light) (Utilities|Struct|MakeLinearColor 1.0 1.0 1.0 1.0))))

(fn ConstructionScript)