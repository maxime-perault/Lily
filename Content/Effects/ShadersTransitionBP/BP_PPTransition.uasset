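; Blueprint that fades the level's look between a Dark and an Oni state.
; SetDark and SetOni raise flags and trigger player-character soundscapes, with a silent variant for Dark.
; When no fade is running, Tick consumes a flag and plays or reverses one Fade timeline.
; Its alpha lerps hardcoded post-process, height fog, directional light and skylight values, though gamma's alpha stays at zero.
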(event EventTick
  (params (DeltaSeconds :type Float%20%28single-precision%29))
  (bind _heightfog (Variables|Default|GetHeightFog))
  (bind _lightsource (Variables|Default|GetLightSource))
  (bind _skylight (Variables|Default|GetSkyLight))
  (bind _component (Variables|/Script/Engine.ExponentialHeightFog|GetComponent _heightfog))
  (bind _lightcomponent (Variables|/Script/Engine.Light|GetLightComponent _lightsource))
  (bind _lightcomponent_2 (Variables|/Script/Engine.SkyLight|GetLightComponent _skylight))
  (if (not (Variables|Default|Getfading))
    (if (Variables|Default|GetisDark)
      (Variables|Default|SetisDark false)
      (Variables|Default|Setfading true)
      (bind _newtrack_0 (Timeline|Fade Play)
        (:Update
          ;[1 1 1] Post Process Volume
          (Utilities|Struct|SetmembersinPostProcessSettings (Variables|/Script/Engine.PostProcessVolume|GetSettings (Variables|Default|GetPostProcessVolume)) (Math|Float|Lerp (Math|Float|MakeLiteralFloat 6.5e+03) (Math|Float|MakeLiteralFloat 2.7e+03) _newtrack_0) (Math|Float|Lerp (Math|Float|MakeLiteralFloat 0.0) (Math|Float|MakeLiteralFloat -0.7) _newtrack_0) (Math|Vector4|MakeVector4 (Math|Float|Lerp 1.0 0.0 _newtrack_0) (Math|Float|Lerp 1.0 0.11 _newtrack_0) (Math|Float|Lerp 1.0 0.24 _newtrack_0) (Math|Float|Lerp 1.0 1.15 _newtrack_0)) (Math|Vector4|MakeVector4 1.0 1.0 1.0 1.0) (Math|Vector4|MakeVector4 (Math|Float|Lerp 1.0 1.1 0.0) (Math|Float|Lerp 1.0 1.2 0.0) (Math|Float|Lerp 1.0 1.2 0.0) (Math|Float|Lerp 1.0 0.5 0.0)) (Math|Float|Lerp (Math|Float|MakeLiteralFloat 0.18) (Math|Float|MakeLiteralFloat 2.5) _newtrack_0) 0.0 0.0 (Math|Float|Lerp (Math|Float|MakeLiteralFloat 0.3) (Math|Float|MakeLiteralFloat 0.7) _newtrack_0) 0.0 (Math|Float|Lerp (Math|Float|MakeLiteralFloat 0.2) (Math|Float|MakeLiteralFloat 0.05) _newtrack_0))
          ;[1 1 1] HeightFog
          (Class|ExponentialHeightFogComponent|SetFogInscatteringColor _component (Utilities|Struct|MakeLinearColor (Math|Float|Lerp 1.0 0.76 _newtrack_0) (Math|Float|Lerp 0.1 1.0 _newtrack_0) (Math|Float|Lerp 0.0 0.94 _newtrack_0) (Math|Float|Lerp 1.0 1.0 _newtrack_0)))
          (Class|ExponentialHeightFogComponent|SetFogDensity _component (Math|Float|Lerp (Math|Float|MakeLiteralFloat 0.02) (Math|Float|MakeLiteralFloat 0.9) _newtrack_0))
          (Class|ExponentialHeightFogComponent|SetFogHeightFalloff _component (Math|Float|Lerp (Math|Float|MakeLiteralFloat 0.1) (Math|Float|MakeLiteralFloat 0.2) _newtrack_0))
          (Class|ExponentialHeightFogComponent|SetStartDistance _component (Math|Float|Lerp (Math|Float|MakeLiteralFloat 5e+03) (Math|Float|MakeLiteralFloat 0.0) _newtrack_0))
          (Class|ExponentialHeightFogComponent|SetDirectionalInscatteringStartDistance _component (Math|Float|Lerp (Math|Float|MakeLiteralFloat 0.0) (Math|Float|MakeLiteralFloat 1e+02) _newtrack_0))
          (Class|ExponentialHeightFogComponent|SetDirectionalInscatteringColor _component (Utilities|Struct|MakeLinearColor (Math|Float|Lerp 1.0 0.02 _newtrack_0) (Math|Float|Lerp 0.14 0.06 _newtrack_0) (Math|Float|Lerp 0.0 0.25 _newtrack_0) (Math|Float|Lerp 1.0 1.0 _newtrack_0)))
          ;[1 1 1] Directional Light
          (Rendering|Components|Light|SetIntensity _lightcomponent (Math|Float|Lerp (Math|Float|MakeLiteralFloat 13.0) (Math|Float|MakeLiteralFloat 2.6) _newtrack_0))
          (Rendering|Components|Light|SetLightColor _lightcomponent (Utilities|Struct|MakeLinearColor (Math|Float|Lerp 1.0 0.527115 _newtrack_0) (Math|Float|Lerp 0.835294 0.806952 _newtrack_0) (Math|Float|Lerp 0.694118 1.0 _newtrack_0) (Math|Float|Lerp 1.0 1.0 _newtrack_0)) true)
          ;[1 1 1] SkyLight
          (Rendering|Components|Light|SetIntensity _lightcomponent_2 (Math|Float|Lerp (Math|Float|MakeLiteralFloat 1.52381) (Math|Float|MakeLiteralFloat 0.19) _newtrack_0))
          (Rendering|Components|Light|SetLightColor _lightcomponent_2 (Utilities|Struct|MakeLinearColor (Math|Float|Lerp 0.835294 1.0 _newtrack_0) (Math|Float|Lerp 0.729412 1.0 _newtrack_0) (Math|Float|Lerp 0.560784 1.0 _newtrack_0) (Math|Float|Lerp 1.0 1.0 _newtrack_0))))
        (:Finished
          (Variables|Default|Setfading false)))
      (elif (Variables|Default|GetisOni)
        (Variables|Default|SetisOni false)
        (Variables|Default|Setfading true)
        (Timeline|Fade Reverse)))))

(fn ConstructionScript)

(fn SetDark
  (bind _asthird_person_character (Utilities|Casting|CastToThirdPersonCharacter (Game|Player|GetPlayerPawn 0)))
  (Default|PlaySoundscapeS1 _asthird_person_character)
  (Variables|Default|SetisDark true))

(fn SetOni
  (bind _asthird_person_character (Utilities|Casting|CastToThirdPersonCharacter (Game|Player|GetPlayerPawn 0)))
  (Default|PlaySoundscapeO1 _asthird_person_character)
  (Variables|Default|SetisOni true))

(fn SetDarkWithoutSound
  (Variables|Default|SetisDark true))