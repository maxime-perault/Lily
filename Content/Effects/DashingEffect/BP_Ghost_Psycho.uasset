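; Short-lived ghost actor for the BP_Psychosis character, apparently an afterimage for the dash effect.
; The construction script caches the first BP_Psychosis found; BeginPlay moves the root to its skeletal mesh location and adds a skeletal mesh component.
; The PlaceGhost timeline drives GhostVisible in the Mpc_dash parameter collection, a value shared globally rather than per ghost, then destroys the actor.
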(event EventBeginPlay
  (Transformation|SetWorldLocation (Variables|Default|GetRoot) (Transformation|GetWorldLocation (Variables|/Game/DarkPhase/Psychosis/BP_Psychosis.BP_Psychosis_C|GetSkeletalMesh (Variables|Default|GetPsychosis))) false false)
  (AddComponent|AddSkeletalMeshComponent false)
  (bind _newtrack_0 (Timeline|Place%20ghost PlayFromStart)
    (:Update
      (Rendering|Material|SetScalarParameterValue "/Game/Effects/DashingEffect/mpc_dash.mpc_dash" "GhostVisible" _newtrack_0 :!class /Script/Engine.KismetMaterialLibrary))
    (:Finished
      (Actor|DestroyActor))))

(fn ConstructionScript
  (bind _outactors (Actor|GetAllActorsOfClass "/Game/DarkPhase/Psychosis/BP_Psychosis.BP_Psychosis_C"))
  (Variables|Default|SetPsychosis (Utilities|Array|Get(acopy) _outactors)))