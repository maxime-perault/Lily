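; Player light zone Blueprint: a spotlight and sphere area that grows on activation, shrinks over time and is refilled by fireflies.
; Tick drives the IncreaseZone and DecreaseZone timelines, which scale cone angles, sphere size and intensity and update HealthZone.
; ReloadFireflies activates the zone or flags a reload, remapping timeline positions from LastTimePercent between shrinking and growing.
; Reset zeroes the zone and stops both timelines; the health bar widget creation is unconnected.
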(event EventTick
  (params (DeltaSeconds :type Float%20%28single-precision%29))
  (bind _spotlight (Variables|Default|GetSpotLight))
  (bind _spotlight_2 (Variables|Default|GetSpotLight))
  ;[1 1 1] Manage Light Zone in S1
  ;;[1 1 1] Decrease the Zone
  (if (Variables|Default|GetisLightZone)
    ;;[1 1 1] Reload with fireflies
    (if (Variables|Default|GetReloading)
      (if (not (Audio|Components|Audio|IsPlaying (Variables|Default|GetIncreaseZone)))
        (if (Variables|Default|GetsettingPosition)
          ;;[1 1 1] Set the last time from decreasing zone
          (Variables|Default|SetsettingPosition false)
          (Components|Timeline|SetPlaybackPosition (Variables|Default|GetIncreaseZone) (- 1.0 (* (Variables|Default|GetlastTimePercent) (/ 1.0 (Components|Timeline|GetTimelineLength (Variables|Default|GetIncreaseZone))))) false true)
          (bind _newtrack_0 (Timeline|IncreaseZone Play)
            (:Update
              (Rendering|Lighting|SetOuterConeAngle _spotlight_2 (* (Variables|Default|Getinitial%20Outer%20corner) _newtrack_0))
              (Rendering|Lighting|SetInnerConeAngle _spotlight_2 (* (Variables|Default|Getinitial%20Inner%20corner) _newtrack_0))
              (Transformation|SetWorldScale3D (Variables|Default|GetSphere) (* (Variables|Default|Getinitial%20sphere%20zone) _newtrack_0))
              (Rendering|Components|Light|SetIntensity _spotlight_2 (* _newtrack_0 (Variables|Default|Getinitial%20Intensity)))
              (bind _output_get (Variables|Default|SetlastTimePercent (/ (Components|Timeline|GetPlaybackPosition (Variables|Default|GetIncreaseZone)) (Components|Timeline|GetTimelineLength (Variables|Default|GetIncreaseZone)))))
              (Variables|Default|SetHealthZone _output_get))
            (:Finished
              (bind _output_get_2 (Variables|Default|SetlastTimePercent (/ (Components|Timeline|GetPlaybackPosition (Variables|Default|GetIncreaseZone)) (Components|Timeline|GetTimelineLength (Variables|Default|GetIncreaseZone)))))
              (Variables|Default|SetHealthZone _output_get_2)
              (if (Variables|Default|GetisLightZone)
                ;;[1 1 1] If the reload of fireflies is finished, set the new time for decreasing zone
                (if (Variables|Default|GetReloading)
                  (Variables|Default|SetReloading false)
                  (bind (_direction _scale _itensity_scale) (Timeline|DecreaseZone SetNewTime)
                    (:Update
                      (Rendering|Lighting|SetOuterConeAngle _spotlight (* (Variables|Default|Getinitial%20Outer%20corner) _scale))
                      (Rendering|Lighting|SetInnerConeAngle _spotlight (* (Variables|Default|Getinitial%20Inner%20corner) _scale))
                      (Transformation|SetWorldScale3D (Variables|Default|GetSphere) (* (Variables|Default|Getinitial%20sphere%20zone) _scale))
                      (Rendering|Components|Light|SetIntensity _spotlight (* _itensity_scale (Variables|Default|Getinitial%20Intensity)))
                      (bind _output_get_3 (Variables|Default|SetlastTimePercent (/ (Components|Timeline|GetPlaybackPosition (Variables|Default|GetDecreaseZone)) (Components|Timeline|GetTimelineLength (Variables|Default|GetDecreaseZone)))))
                      (Variables|Default|SetHealthZone (- 1.0 _output_get_3)))))
                (else
                  ;;[1 1 1] Start Zone HUD
                  (Variables|Default|SetisLightZone true)))))))
      (elif (not (Audio|Components|Audio|IsPlaying (Variables|Default|GetDecreaseZone)))
        (Timeline|DecreaseZone Play)))
    (else
      ;;[1 1 1] Start the Zone
      (if (Variables|Default|GetActivateZone)
        (if (not (Audio|Components|Audio|IsPlaying (Variables|Default|GetIncreaseZone)))
          (Timeline|IncreaseZone Play))))))

(fn ConstructionScript)

(fn ReloadFireflies
  (if (Variables|Default|GetActivateZone)
    (Variables|Default|SetReloading true)
    (Variables|Default|SetsettingPosition true)
    (Variables|Default|SetlastTimePercent (/ (Components|Timeline|GetPlaybackPosition (Variables|Default|GetDecreaseZone)) (Components|Timeline|GetTimelineLength (Variables|Default|GetDecreaseZone))))
    (else
      (Variables|Default|SetActivateZone true))))

(fn EnableLightingZone
  (Variables|Default|SetActivateZone true))

(fn Reset
  (bind _spotlight (Variables|Default|GetSpotLight))
  (Variables|Default|SetisLightZone false)
  (Variables|Default|SetActivateZone false)
  (Variables|Default|SetReloading false)
  (Variables|Default|SetsettingPosition false)
  (Variables|Default|SetlastTimePercent 0.0)
  (Variables|Default|SetHealthZone 0.0)
  (Rendering|Lighting|SetOuterConeAngle _spotlight 0.0)
  (Rendering|Lighting|SetInnerConeAngle _spotlight 0.0)
  (Transformation|SetWorldScale3D (Variables|Default|GetSphere) "0, 0, 0")
  (Rendering|Components|Light|SetIntensity _spotlight 0.0)
  (Audio|Components|Audio|Stop (Variables|Default|GetIncreaseZone))
  (Audio|Components|Audio|Stop (Variables|Default|GetDecreaseZone)))