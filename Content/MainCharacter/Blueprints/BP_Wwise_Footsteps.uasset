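; Actor Blueprint that keeps the Wwise "Footsteps" switch matched to the surface under the player.
; Each tick, unless IsWater is set, it line-traces down from the player pawn and reads the physical surface type.
; Only when the surface changes, it sets the matching switch state on the AkComponent of the ThirdPersonCharacter's mesh.
; It only selects the switch and posts no sound events itself.
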(event EventTick
  (params (DeltaSeconds :type Float%20%28single-precision%29))
  (bind _returnvalue (Game|Player|GetPlayerPawn 0))
  (bind _returnvalue_2 (Transformation|GetActorLocation _returnvalue))
  (if (not (Variables|Default|GetisWater))
    (bind (_outhit _returnvalue_3) (Collision|LineTraceByChannel _returnvalue_2 (- _returnvalue_2 "0, 0,100.000000") "TraceTypeQuery1" false 0 "None" false))
    (if _returnvalue_3
      (if (not (== (Collision|GetSurfaceType _outhit) (Variables|Default|GetCurrent%20Surface%20Type)))
        (bind _output_get (Variables|Default|SetCurrent%20Surface%20Type (Collision|GetSurfaceType _outhit)))
        (bind _asthird_person_character (Utilities|Casting|CastToThirdPersonCharacter (Game|Player|GetPlayerPawn 0)))
        (bind _returnvalue_4 (Class|AkGameplayStatics|GetAkComponent (Variables|/Script/Engine.Character|GetMesh _asthird_person_character) "None" "0, 0, 0" "KeepRelativeOffset"))
        (switch string (Utilities|String|ToString(Byte) _output_get)
          (:1
            (Class|AkComponent|SetSwitch _returnvalue_4 "Footsteps" "Dirt"))
          (:2
            (Class|AkComponent|SetSwitch _returnvalue_4 "Footsteps" "Grass"))
          (:3
            (Class|AkComponent|SetSwitch _returnvalue_4 "Footsteps" "Water"))
          (:4
            (Class|AkComponent|SetSwitch _returnvalue_4 "Footsteps" "Wood"))
          (:5
            (Class|AkComponent|SetSwitch _returnvalue_4 "Footsteps" "Rocks"))
          (:6
            (Class|AkComponent|SetSwitch _returnvalue_4 "Footsteps" "Flowers"))
          (:7
            (Class|AkComponent|SetSwitch _returnvalue_4 "Footsteps" "Mirror"))
          (:8
            (Class|AkComponent|SetSwitch _returnvalue_4 "Footsteps" "Roots")))))))

(fn ConstructionScript)