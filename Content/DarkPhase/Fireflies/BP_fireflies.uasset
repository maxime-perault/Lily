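; BP_fireflies is a firefly pickup that reloads the fireflies of the player's LightingZone.
; It plays a looping-style Wwise idle sound until the player overlaps its Box, then stops it and calls ReloadFireflies on the LightingZone, found at a fixed index among the player's child actors.
; The pickup then disables collision and hides its light and orbiting fireflies rather than being destroyed, so Reset can restore them and restart the sound.
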(event OnComponentBeginOverlap(Box)
  (params (OverlappedComponent :type Primitive%20Component%20Object%20Reference) (OtherActor :type Actor%20Object%20Reference) (OtherComp :type Primitive%20Component%20Object%20Reference) (OtherBodyIndex :type Integer) (bFromSweep :type Boolean) (SweepResult :type Hit%20Result%20Structure%20%28by%20ref%29))
  (bind _player (Variables|Default|GetPlayer))
  (if (== OtherActor _player)
    (Class|AkGameplayStatics|PostEvent "/Game/Wwise/Stop_Fireflies_idle.Stop_Fireflies_idle" self false)
    (bind _aslighting_zone (Utilities|Casting|CastToLightingZone (Utilities|Array|Get(acopy) (Actor|GetAllChildActors _player true) 1)))
    (Default|ReloadFireflies _aslighting_zone)
    (Collision|SetCollisionEnabled (Variables|Default|GetBox) "NoCollision")
    (Rendering|SetVisibility (Variables|Default|GetPointLight) false false)
    (Rendering|SetVisibility (Variables|Default|GetP_orbitFireflies) false false)))

(event EventBeginPlay
  (Variables|Default|SetPlayer (Game|GetPlayerCharacter 0))
  (Class|AkGameplayStatics|PostEvent "/Game/Wwise/Play_Fireflies_idle.Play_Fireflies_idle" self false))

(fn ConstructionScript)

(fn Reset
  (Collision|SetCollisionEnabled (Variables|Default|GetBox) "QueryOnly")
  (Rendering|SetVisibility (Variables|Default|GetPointLight) true false)
  (Rendering|SetVisibility (Variables|Default|GetP_orbitFireflies) true false)
  (Class|AkGameplayStatics|PostEvent "/Game/Wwise/Play_Fireflies_idle.Play_Fireflies_idle" self false))