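; BP_Outro is a trigger actor for the outro that fires when the player overlaps its Trigger component.
; It caches the first BP_Psychosis in the level on BeginPlay.
; On overlap it disables the trigger's collision, calls Fix on the Mirror and zeroes PsychosisVisible in the Mpc_dash material parameter collection.
; It then spawns a BP_Ghost_Psycho at the cached Psychosis actor's transform.
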(event OnComponentBeginOverlap(trigger)
  (params (OverlappedComponent :type Primitive%20Component%20Object%20Reference) (OtherActor :type Actor%20Object%20Reference) (OtherComp :type Primitive%20Component%20Object%20Reference) (OtherBodyIndex :type Integer) (bFromSweep :type Boolean) (SweepResult :type Hit%20Result%20Structure%20%28by%20ref%29))
  (if (== OtherActor (Game|GetPlayerCharacter 0))
    (Collision|SetCollisionEnabled (Variables|Default|Gettrigger) "NoCollision")
    (Default|Fix (Variables|Default|GetMirror))
    (Rendering|Material|SetScalarParameterValue "/Game/Effects/DashingEffect/mpc_dash.mpc_dash" "PsychosisVisible" 0.0 :!class /Script/Engine.KismetMaterialLibrary)
    (Game|SpawnActorfromClass "/Game/Effects/DashingEffect/BP_Ghost_Psycho.BP_Ghost_Psycho_C" (Transformation|GetActorTransform (Variables|Default|GetPsychosis)) "Undefined" 0 0)))

(event EventBeginPlay
  (bind _outactors (Actor|GetAllActorsOfClass "/Game/DarkPhase/Psychosis/BP_Psychosis.BP_Psychosis_C"))
  (Variables|Default|SetPsychosis (Utilities|Array|Get(acopy) _outactors)))

(fn ConstructionScript)