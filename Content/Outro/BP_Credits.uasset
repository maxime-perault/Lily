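; Trigger actor that plays the end-game credits when the player character walks into it.
; On first overlap it disables its trigger collision, then creates a W_OutroScreen widget and adds it to the viewport.
; A hardcoded chain of delays calls LaunchMessage for each role title and team member name, with larger text for titles and timed fades.
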(event OnComponentBeginOverlap(Trigger)
  (params (OverlappedComponent :type Primitive%20Component%20Object%20Reference) (OtherActor :type Actor%20Object%20Reference) (OtherComp :type Primitive%20Component%20Object%20Reference) (OtherBodyIndex :type Integer) (bFromSweep :type Boolean) (SweepResult :type Hit%20Result%20Structure%20%28by%20ref%29))
  (if (== OtherActor (Game|GetPlayerCharacter 0))
    (Collision|SetCollisionEnabled (Variables|Default|GetTrigger) "NoCollision")
    (bind _returnvalue (UserInterface|CreateWidget "/Game/Outro/W_OutroScreen.W_OutroScreen_C" (Game|GetPlayerController 0)))
    (UserInterface|Viewport|AddtoViewport _returnvalue 0)
    (Default|LaunchMessage _returnvalue "Producer" 40 4.0)
    (Utilities|FlowControl|Delay 0.5)
    (Default|LaunchMessage _returnvalue "William Désert" 20 3.0)
    (Utilities|FlowControl|Delay 4.0)
    (Default|LaunchMessage _returnvalue "Programmer" 40 4.0)
    (Utilities|FlowControl|Delay 0.5)
    (Default|LaunchMessage _returnvalue "Maxime Perault" 20 3.0)
    (Utilities|FlowControl|Delay 4.0)
    (Default|LaunchMessage _returnvalue "3D Artist" 40 4.0)
    (Utilities|FlowControl|Delay 0.5)
    (Default|LaunchMessage _returnvalue "Lise Sourlier" 20 3.0)
    (Utilities|FlowControl|Delay 4.0)
    (Default|LaunchMessage _returnvalue "Game Design" 40 4.0)
    (Utilities|FlowControl|Delay 0.5)
    (Default|LaunchMessage _returnvalue "Victor Girard" 20 3.0)
    (Utilities|FlowControl|Delay 0.1)
    (Default|LaunchMessage _returnvalue "Maxime Perault" 20 3.0)
    (Utilities|FlowControl|Delay 4.1)
    (Default|LaunchMessage _returnvalue "UI/UX Designer" 40 4.0)
    (Utilities|FlowControl|Delay 0.5)
    (Default|LaunchMessage _returnvalue "Anaïtis de France" 20 3.0)
    (Utilities|FlowControl|Delay 4.0)
    (Default|LaunchMessage _returnvalue "Sound Design" 40 4.0)
    (Utilities|FlowControl|Delay 0.5)
    (Default|LaunchMessage _returnvalue "Robin Richard" 20 3.0)))

(fn ConstructionScript)