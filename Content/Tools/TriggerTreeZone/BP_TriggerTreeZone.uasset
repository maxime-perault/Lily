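; BP_TriggerTreeZone is a one-shot trigger zone that fires tree zone feedback and a voice line when the player enters it.
; On first player overlap, the TriggerSound component disables its own collision, then calls PlayTreeZone on the ThirdPersonCharacter.
; After a short delay, it posts the Wwise event Voiceline_Grotte_1 on itself.
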(event OnComponentBeginOverlap(TriggerSound)
  (params (OverlappedComponent :type Primitive%20Component%20Object%20Reference) (OtherActor :type Actor%20Object%20Reference) (OtherComp :type Primitive%20Component%20Object%20Reference) (OtherBodyIndex :type Integer) (bFromSweep :type Boolean) (SweepResult :type Hit%20Result%20Structure%20%28by%20ref%29))
  (if (== OtherActor (Variables|Default|GetPlayer))
    (Collision|SetCollisionEnabled (Variables|Default|GetTriggerSound) "NoCollision")
    (bind _asthird_person_character (Utilities|Casting|CastToThirdPersonCharacter (Game|Player|GetPlayerPawn 0)))
    (Default|PlayTreeZone _asthird_person_character)
    (Utilities|FlowControl|Delay 3.0)
    (Class|AkGameplayStatics|PostEvent "/Game/Wwise/Voiceline_Grotte_1.Voiceline_Grotte_1" self false)))

(event EventBeginPlay
  (Variables|Default|SetPlayer (Game|GetPlayerCharacter 0)))

(fn ConstructionScript)