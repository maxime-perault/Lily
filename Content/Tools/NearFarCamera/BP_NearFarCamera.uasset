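; BP_NearFarCamera is a trigger-pair actor that switches the player's camera between far and near framing, along with the ambiance.
; Overlapping TriggerIn plays the Fade timeline, shortening and lowering the ThirdPersonCharacter's camera boom; TriggerOut reverses it.
; Each trigger also sets the first BP_switchAMB's state and passes it to the character's SwitchAmbiance.
; In/Out flags block repeat triggers, with IsOut influencing their initial values at construction.
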(event OnComponentBeginOverlap(TriggerIn)
  (params (OverlappedComponent :type Primitive%20Component%20Object%20Reference) (OtherActor :type Actor%20Object%20Reference) (OtherComp :type Primitive%20Component%20Object%20Reference) (OtherBodyIndex :type Integer) (bFromSweep :type Boolean) (SweepResult :type Hit%20Result%20Structure%20%28by%20ref%29))
  (bind _player (Variables|Default|GetPlayer))
  (bind _cameraboom (Variables|/Game/MainCharacter/Blueprints/ThirdPersonCharacter.ThirdPersonCharacter_C|GetCameraBoom _player))
  (bind _relativelocation (Variables|/Script/Engine.SceneComponent|GetRelativeLocation _cameraboom))
  (bind (_x _y) (Math|Vector|BreakVector _relativelocation))
  (if (== (Variables|Default|GetPlayer) OtherActor)
    (if (not (Variables|Default|GetIn))
      (Variables|Default|SetIn true)
      (Variables|Default|SetOut false)
      (bind _asthird_person_character (Utilities|Casting|CastToThirdPersonCharacter (Game|Player|GetPlayerPawn 0)))
      (bind _outactors (Actor|GetAllActorsOfClass "/Game/Wwise/WwiseBP/BP_switchAMB.BP_switchAMB_C"))
      (bind _output_get (Variables|/Game/Wwise/WwiseBP/BP_switchAMB.BP_switchAMB_C|SetcurrentState (Utilities|Array|Get(acopy) _outactors) 4))
      (Default|SwitchAmbiance _asthird_person_character _output_get)
      (bind _newtrack_0 (Timeline|Fade PlayFromStart)
        (:Update
          (Variables|/Script/Engine.SpringArmComponent|SetTargetArmLength _cameraboom (Math|Float|Lerp (Math|Float|MakeLiteralFloat 5e+02) (Math|Float|MakeLiteralFloat 2e+02) _newtrack_0))
          (Transformation|SetRelativeLocation _cameraboom (Math|Vector|MakeVector _x _y (Math|Float|Lerp (Variables|Default|GetOut_z_cam) (Variables|Default|GetIn_Z_cam) _newtrack_0)) false false))))))

(event OnComponentBeginOverlap(TriggerOut)
  (params (OverlappedComponent :type Primitive%20Component%20Object%20Reference) (OtherActor :type Actor%20Object%20Reference) (OtherComp :type Primitive%20Component%20Object%20Reference) (OtherBodyIndex :type Integer) (bFromSweep :type Boolean) (SweepResult :type Hit%20Result%20Structure%20%28by%20ref%29))
  (bind _player (Variables|Default|GetPlayer))
  (bind _cameraboom (Variables|/Game/MainCharacter/Blueprints/ThirdPersonCharacter.ThirdPersonCharacter_C|GetCameraBoom _player))
  (bind _relativelocation (Variables|/Script/Engine.SceneComponent|GetRelativeLocation _cameraboom))
  (bind (_x _y) (Math|Vector|BreakVector _relativelocation))
  (if (== (Variables|Default|GetPlayer) OtherActor)
    (if (not (Variables|Default|GetOut))
      (Variables|Default|SetOut true)
      (Variables|Default|SetIn false)
      (bind _asthird_person_character (Utilities|Casting|CastToThirdPersonCharacter (Game|Player|GetPlayerPawn 0)))
      (bind _outactors (Actor|GetAllActorsOfClass "/Game/Wwise/WwiseBP/BP_switchAMB.BP_switchAMB_C"))
      (bind _output_get (Variables|/Game/Wwise/WwiseBP/BP_switchAMB.BP_switchAMB_C|SetcurrentState (Utilities|Array|Get(acopy) _outactors) 2))
      (Default|SwitchAmbiance _asthird_person_character _output_get)
      (bind _newtrack_0 (Timeline|Fade ReverseFromEnd)
        (:Update
          (Variables|/Script/Engine.SpringArmComponent|SetTargetArmLength _cameraboom (Math|Float|Lerp (Math|Float|MakeLiteralFloat 5e+02) (Math|Float|MakeLiteralFloat 2e+02) _newtrack_0))
          (Transformation|SetRelativeLocation _cameraboom (Math|Vector|MakeVector _x _y (Math|Float|Lerp (Variables|Default|GetOut_z_cam) (Variables|Default|GetIn_Z_cam) _newtrack_0)) false false))))))

(event EventBeginPlay
  (bind _asthird_person_character (Utilities|Casting|CastToThirdPersonCharacter (Game|GetPlayerCharacter 0)))
  (bind _output_get (Variables|Default|SetPlayer _asthird_person_character))
  (bind _output_get_2 (Variables|Default|SetOut_z_cam (.Z (Math|Vector|BreakVector (Variables|/Script/Engine.SceneComponent|GetRelativeLocation (Variables|/Game/MainCharacter/Blueprints/ThirdPersonCharacter.ThirdPersonCharacter_C|GetCameraBoom _output_get))))))
  (Variables|Default|SetIn_Z_cam (- _output_get_2 3e+01)))

(fn ConstructionScript
  (if (not (Variables|Default|GetIsOut))
    (Variables|Default|SetIn true)
    (Variables|Default|SetOut false)))