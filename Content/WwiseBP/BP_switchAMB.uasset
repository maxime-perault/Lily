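; BP_switchAMB is a trigger actor that switches the player's ambiance as they move in and out of Cabin 1 through its top and bottom sides.
; Four overlap components map to three states: inside from either side, exited at the top, and exited at the bottom.
; On a state change it stores CurrentState and calls SwitchAmbiance on the player's ThirdPersonCharacter, without checking which actor overlapped.
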(event OnComponentBeginOverlap(EnterCabin1FromBot)
  (params (OverlappedComponent :type Primitive%20Component%20Object%20Reference) (OtherActor :type Actor%20Object%20Reference) (OtherComp :type Primitive%20Component%20Object%20Reference) (OtherBodyIndex :type Integer) (bFromSweep :type Boolean) (SweepResult :type Hit%20Result%20Structure%20%28by%20ref%29))
  (if (!= (Variables|Default|GetcurrentState) 1)
    (bind _asthird_person_character (Utilities|Casting|CastToThirdPersonCharacter (Game|Player|GetPlayerPawn 0)))
    (bind _output_get (Variables|Default|SetcurrentState 1))
    (Default|SwitchAmbiance _asthird_person_character _output_get)))

(event OnComponentBeginOverlap(ExitCabin1FromBot)
  (params (OverlappedComponent :type Primitive%20Component%20Object%20Reference) (OtherActor :type Actor%20Object%20Reference) (OtherComp :type Primitive%20Component%20Object%20Reference) (OtherBodyIndex :type Integer) (bFromSweep :type Boolean) (SweepResult :type Hit%20Result%20Structure%20%28by%20ref%29))
  (if (!= (Variables|Default|GetcurrentState) 0)
    (bind _asthird_person_character (Utilities|Casting|CastToThirdPersonCharacter (Game|Player|GetPlayerPawn 0)))
    (Variables|Default|SetcurrentState 0)
    (Default|SwitchAmbiance _asthird_person_character)))

(event OnComponentBeginOverlap(EnterCabin1FromTop)
  (params (OverlappedComponent :type Primitive%20Component%20Object%20Reference) (OtherActor :type Actor%20Object%20Reference) (OtherComp :type Primitive%20Component%20Object%20Reference) (OtherBodyIndex :type Integer) (bFromSweep :type Boolean) (SweepResult :type Hit%20Result%20Structure%20%28by%20ref%29))
  (if (!= (Variables|Default|GetcurrentState) 1)
    (bind _asthird_person_character (Utilities|Casting|CastToThirdPersonCharacter (Game|Player|GetPlayerPawn 0)))
    (bind _output_get (Variables|Default|SetcurrentState 1))
    (Default|SwitchAmbiance _asthird_person_character _output_get)))

(event OnComponentBeginOverlap(ExitCabin1FromTop)
  (params (OverlappedComponent :type Primitive%20Component%20Object%20Reference) (OtherActor :type Actor%20Object%20Reference) (OtherComp :type Primitive%20Component%20Object%20Reference) (OtherBodyIndex :type Integer) (bFromSweep :type Boolean) (SweepResult :type Hit%20Result%20Structure%20%28by%20ref%29))
  (if (!= (Variables|Default|GetcurrentState) 2)
    (bind _asthird_person_character (Utilities|Casting|CastToThirdPersonCharacter (Game|Player|GetPlayerPawn 0)))
    (bind _output_get (Variables|Default|SetcurrentState 2))
    (Default|SwitchAmbiance _asthird_person_character _output_get)))

(fn ConstructionScript)