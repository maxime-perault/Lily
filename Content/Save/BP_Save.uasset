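; BP_Save is a one-shot checkpoint trigger that records a save position on the player character.
; It caches player pawn 0 on BeginPlay and compares it against actors that begin overlapping its Box component.
; On a match, it casts the pawn to ThirdPersonCharacter, copies its SaveCheckpoint value into the character's SavePos, then destroys itself.
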(event OnComponentBeginOverlap(Box)
  (params (OverlappedComponent :type Primitive%20Component%20Object%20Reference) (OtherActor :type Actor%20Object%20Reference) (OtherComp :type Primitive%20Component%20Object%20Reference) (OtherBodyIndex :type Integer) (bFromSweep :type Boolean) (SweepResult :type Hit%20Result%20Structure%20%28by%20ref%29))
  (if (== OtherActor (Variables|Default|GetPlayer))
    (bind _asthird_person_character (Utilities|Casting|CastToThirdPersonCharacter (Variables|Default|GetPlayer)))
    (Variables|/Game/ThirdPersonBP/Blueprints/ThirdPersonCharacter.ThirdPersonCharacter_C|SetSave_Pos _asthird_person_character (Variables|Default|GetSave_Checkpoint))
    (Actor|DestroyActor)))

(event EventBeginPlay
  (Variables|Default|SetPlayer (Game|Player|GetPlayerPawn 0)))

(fn ConstructionScript)