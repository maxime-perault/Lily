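; Trigger-volume actor that switches Wwise ambience as the player enters and exits two cabins from top or bottom.
; Each overlap updates CurrentState, skipping repeats, and passes it to ThirdPersonCharacter's SwitchAmbiance.
; Some crossings, mostly at the top, also start or stop soundscape events on the character.
; Two one-shot voicelines play: one flag-guarded on Cabin 1's bottom entry, another from PaintVoiceline, which disables its collision.
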(event OnComponentBeginOverlap(EnterCabin2FromBot)
  (params (OverlappedComponent :type Primitive%20Component%20Object%20Reference) (OtherActor :type Actor%20Object%20Reference) (OtherComp :type Primitive%20Component%20Object%20Reference) (OtherBodyIndex :type Integer) (bFromSweep :type Boolean) (SweepResult :type Hit%20Result%20Structure%20%28by%20ref%29))
  ;[1 1 1] 2nd Cabin
  (if (== (Game|GetPlayerCharacter 0) OtherActor)
    (if (!= (Variables|Default|GetcurrentState) 3)
      (bind _asthird_person_character (Utilities|Casting|CastToThirdPersonCharacter (Game|Player|GetPlayerPawn 0)))
      (bind _output_get (Variables|Default|SetcurrentState 3))
      (Default|SwitchAmbiance _asthird_person_character _output_get))))

(event OnComponentBeginOverlap(EnterCabin1FromBot)
  (params (OverlappedComponent :type Primitive%20Component%20Object%20Reference) (OtherActor :type Actor%20Object%20Reference) (OtherComp :type Primitive%20Component%20Object%20Reference) (OtherBodyIndex :type Integer) (bFromSweep :type Boolean) (SweepResult :type Hit%20Result%20Structure%20%28by%20ref%29))
  ;[1 1 1] 1st Cabin
  (if (== (Game|GetPlayerCharacter 0) OtherActor)
    (if (!= (Variables|Default|GetcurrentState) 1)
      (bind _asthird_person_character (Utilities|Casting|CastToThirdPersonCharacter (Game|Player|GetPlayerPawn 0)))
      (bind _output_get (Variables|Default|SetcurrentState 1))
      (Default|SwitchAmbiance _asthird_person_character _output_get)
      (if (not (Variables|Default|Getcabin_voiceline_triggered))
        (Variables|Default|Setcabin_voiceline_triggered true)
        (Class|AkGameplayStatics|PostEvent "/Game/Wwise/Voiceline_O1_5.Voiceline_O1_5" _asthird_person_character false)))))

(event OnComponentBeginOverlap(ExitCabin1FromBot)
  (params (OverlappedComponent :type Primitive%20Component%20Object%20Reference) (OtherActor :type Actor%20Object%20Reference) (OtherComp :type Primitive%20Component%20Object%20Reference) (OtherBodyIndex :type Integer) (bFromSweep :type Boolean) (SweepResult :type Hit%20Result%20Structure%20%28by%20ref%29))
  ;[1 1 1] 1st Cabin
  (if (== (Game|GetPlayerCharacter 0) OtherActor)
    (if (!= (Variables|Default|GetcurrentState) 0)
      (bind _asthird_person_character (Utilities|Casting|CastToThirdPersonCharacter (Game|Player|GetPlayerPawn 0)))
      (bind _output_get (Variables|Default|SetcurrentState 0))
      (Default|SwitchAmbiance _asthird_person_character _output_get))))

(event OnComponentBeginOverlap(ExitCabin2FromBot)
  (params (OverlappedComponent :type Primitive%20Component%20Object%20Reference) (OtherActor :type Actor%20Object%20Reference) (OtherComp :type Primitive%20Component%20Object%20Reference) (OtherBodyIndex :type Integer) (bFromSweep :type Boolean) (SweepResult :type Hit%20Result%20Structure%20%28by%20ref%29))
  ;[1 1 1] 2nd Cabin
  (if (== (Game|GetPlayerCharacter 0) OtherActor)
    (if (!= (Variables|Default|GetcurrentState) 2)
      (bind _asthird_person_character (Utilities|Casting|CastToThirdPersonCharacter (Game|Player|GetPlayerPawn 0)))
      (bind _output_get (Variables|Default|SetcurrentState 2))
      (Default|SwitchAmbiance _asthird_person_character _output_get))))

(event OnComponentBeginOverlap(PaintVoiceline)
  (params (OverlappedComponent :type Primitive%20Component%20Object%20Reference) (OtherActor :type Actor%20Object%20Reference) (OtherComp :type Primitive%20Component%20Object%20Reference) (OtherBodyIndex :type Integer) (bFromSweep :type Boolean) (SweepResult :type Hit%20Result%20Structure%20%28by%20ref%29))
  (bind _returnvalue (Game|GetPlayerCharacter 0))
  (if (== _returnvalue OtherActor)
    (Collision|SetCollisionEnabled (Variables|Default|GetPaintVoiceline) "NoCollision")
    (bind _asthird_person_character (Utilities|Casting|CastToThirdPersonCharacter _returnvalue))
    (Class|AkGameplayStatics|PostEvent "/Game/Wwise/Voiceline_O1_3.Voiceline_O1_3" _asthird_person_character false)))

(event OnComponentBeginOverlap(EnterCabin2FromTop)
  (params (OverlappedComponent :type Primitive%20Component%20Object%20Reference) (OtherActor :type Actor%20Object%20Reference) (OtherComp :type Primitive%20Component%20Object%20Reference) (OtherBodyIndex :type Integer) (bFromSweep :type Boolean) (SweepResult :type Hit%20Result%20Structure%20%28by%20ref%29))
  ;[1 1 1] 2nd Cabin
  (if (== (Game|GetPlayerCharacter 0) OtherActor)
    (if (!= (Variables|Default|GetcurrentState) 3)
      (bind _asthird_person_character (Utilities|Casting|CastToThirdPersonCharacter (Game|Player|GetPlayerPawn 0)))
      (bind _output_get (Variables|Default|SetcurrentState 3))
      (Default|SwitchAmbiance _asthird_person_character _output_get)
      (Class|AkGameplayStatics|PostEvent "/Game/Wwise/Stop_Soundscape_Marelle.Stop_Soundscape_Marelle" _asthird_person_character false)
      (Class|AkGameplayStatics|PostEvent "/Game/Wwise/Play_Soundscape_S1.Play_Soundscape_S1" _asthird_person_character false)
      (Class|AkGameplayStatics|PostEvent "/Game/Wwise/Play_Soundscape_Cabane2.Play_Soundscape_Cabane2" _asthird_person_character false))))

(event OnComponentBeginOverlap(ExitCabin2FromTop)
  (params (OverlappedComponent :type Primitive%20Component%20Object%20Reference) (OtherActor :type Actor%20Object%20Reference) (OtherComp :type Primitive%20Component%20Object%20Reference) (OtherBodyIndex :type Integer) (bFromSweep :type Boolean) (SweepResult :type Hit%20Result%20Structure%20%28by%20ref%29))
  ;[1 1 1] 2nd Cabin
  (if (== (Game|GetPlayerCharacter 0) OtherActor)
    (if (!= (Variables|Default|GetcurrentState) 2)
      (bind _asthird_person_character (Utilities|Casting|CastToThirdPersonCharacter (Game|Player|GetPlayerPawn 0)))
      (bind _output_get (Variables|Default|SetcurrentState 2))
      (Default|SwitchAmbiance _asthird_person_character _output_get)
      (Class|AkGameplayStatics|PostEvent "/Game/Wwise/Stop_Soundscape_Cabane2.Stop_Soundscape_Cabane2" _asthird_person_character false)
      (Class|AkGameplayStatics|PostEvent "/Game/Wwise/Stop_Soundscape_S1.Stop_Soundscape_S1" _asthird_person_character false))))

(event OnComponentBeginOverlap(EnterCabin1FromTop)
  (params (OverlappedComponent :type Primitive%20Component%20Object%20Reference) (OtherActor :type Actor%20Object%20Reference) (OtherComp :type Primitive%20Component%20Object%20Reference) (OtherBodyIndex :type Integer) (bFromSweep :type Boolean) (SweepResult :type Hit%20Result%20Structure%20%28by%20ref%29))
  ;[1 1 1] 1st Cabin
  (if (== (Game|GetPlayerCharacter 0) OtherActor)
    (if (!= (Variables|Default|GetcurrentState) 1)
      (bind _asthird_person_character (Utilities|Casting|CastToThirdPersonCharacter (Game|Player|GetPlayerPawn 0)))
      (bind _output_get (Variables|Default|SetcurrentState 1))
      (Default|SwitchAmbiance _asthird_person_character _output_get)
      (Class|AkGameplayStatics|PostEvent "/Game/Wwise/Play_Soundscape_O1.Play_Soundscape_O1" _asthird_person_character false))))

(event OnComponentBeginOverlap(ExitCabin1FromTop)
  (params (OverlappedComponent :type Primitive%20Component%20Object%20Reference) (OtherActor :type Actor%20Object%20Reference) (OtherComp :type Primitive%20Component%20Object%20Reference) (OtherBodyIndex :type Integer) (bFromSweep :type Boolean) (SweepResult :type Hit%20Result%20Structure%20%28by%20ref%29))
  ;[1 1 1] 1st Cabin
  (if (== (Game|GetPlayerCharacter 0) OtherActor)
    (if (!= (Variables|Default|GetcurrentState) 2)
      (bind _asthird_person_character (Utilities|Casting|CastToThirdPersonCharacter (Game|Player|GetPlayerPawn 0)))
      (bind _output_get (Variables|Default|SetcurrentState 2))
      (Default|SwitchAmbiance _asthird_person_character _output_get)
      (Class|AkGameplayStatics|PostEvent "/Game/Wwise/Stop_Soundscape_O1.Stop_Soundscape_O1" _asthird_person_character false))))

(fn ConstructionScript)